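; Bomberman bomb actor that explodes once, on a timer or through its Destroy function, then notifies its instigator and removes itself.
; Explode fires four blasts along GameState axes, each an authority-only sphere trace sending DestroyMessage until an indestructible object or destructible wall stops it.
; DrawBlastParticle stretches a beam emitter to that endpoint.
; The mesh starts blocking pawns once the instigator steps off; BlastInDirection is an unused duplicate.
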(event `self.ReceiveBeginPlay`
  ;[0.1251 0.88 0.01692] Start Bomb timer
  (`KismetSystemLibrary.K2_SetTimer` null "Explode" (`self.Bomb Delay Time`)))

(event `Blast In Direction Replicated`
  (params (Direction :type "Vector Structure"))
  (bind _returnvalue (`SceneComponent.K2_GetComponentLocation` (`self.Bomb Mesh`)))
  (bind _returnvalue_2 (+ _returnvalue (* Direction (`self.Blast Length`))))
  ;[1 1 1] Trace blast in direction
  (`/Engine/EditorBlueprintResources/ActorMacros.Switch Has Authority`
    (:`Authority`
      (`|ExecutionSequence`
        (:`then_0`
          (set `self.Is Destructible Wall` false)
          (set `self._Last Hit Actor Location` (0.0 0.0 0.0))
          (set `self.Hit Object Idx` -1))
        (:`then_1`
          (bind _outhits (`KismetSystemLibrary.SphereTraceMultiForObjects` :`Start` _returnvalue :`End` _returnvalue_2 :`Radius` 10.0 :`ObjectTypes` (`|MakeArray` "ObjectTypeQuery6" "ObjectTypeQuery8" "ObjectTypeQuery7" "ObjectTypeQuery3" :!type "EObjectTypeQuery Enum") :`DrawTime` 1.0))
          (for (_array_element _array_index) _outhits
            (bind (_bblockinghit _binitialoverlap _time _distance _location _impactpoint _normal _impactnormal _physmat _hitactor) (`GameplayStatics.BreakHitResult` _array_element))
            (bind _output_get (set `self.Is Destructible Wall` (`.bSuccess` (cast `/Game/Blueprints/MapConstruction/DestructibleWall` _hitactor :!pure true)))) ; NOTE: Set it before interface call
            (if _output_get
              (set `self._Last Hit Actor Location` (+ _location (* Direction 50.0)))
              (else
                (set `self._Last Hit Actor Location` _location)))
            (bind _success (message `/Game/Blueprints/Weapon/WeaponInteract_Interface.Destroy` _hitactor))
            (if (or (not _success) (`self.Is Destructible Wall`))
              (set `self.Hit Object Idx` _array_index)
              (break)))
          (`self.Draw Blast Particle` (`self.Hit Object Idx`) (`self._Last Hit Actor Location`) _returnvalue _returnvalue_2))))))

(event `Explode`
  (bind _returnvalue (`self.GetInstigator`))
  ;[1 1 1] Explode Bomb
  (`/Engine/EditorBlueprintResources/StandardMacros.DoOnce` false
    (:`Completed`
      (`|ExecutionSequence`
        (:`then_0`
          ;;[1 1 1] Disable sparks, hide Bomb
          (`ActorComponent.Deactivate` (`self.Sparks`))
          (`SceneComponent.SetHiddenInGame` (`self.Bomb Mesh`) true false))
        (:`then_1`
          ;;[1 1 1] Calculate blasts
          (bind _asbomberman_game_state (cast `/Game/Blueprints/GameMode/Bomberman_GameState` (`GameplayStatics.GetGameState`))
            (:`then`
              _)
            (:`CastFailed`
              _))
          (`|ExecutionSequence`
            (:`then_0`
              (bind _world_forward (`/Game/Blueprints/GameMode/Bomberman_GameState.World Forward` _asbomberman_game_state))
              (`self.Blast In Direction Replicated` _world_forward) ; Forward Blast
            )
            (:`then_1`
              (`self.Blast In Direction Replicated` (* _world_forward -1.0)) ; Backward Blast
            )
            (:`then_2`
              (bind _world_right (`/Game/Blueprints/GameMode/Bomberman_GameState.World Right` _asbomberman_game_state))
              (`self.Blast In Direction Replicated` _world_right) ; Right Blast
            )
            (:`then_3`
              (`self.Blast In Direction Replicated` (* _world_right -1.0)) ; Left Blast
            )))
        (:`then_2`
          ;;[1 1 1] Remove Actor
          (`KismetSystemLibrary.Delay` 1.0) ; Wait before removing Actor
          (`|ExecutionSequence`
            (:`then_0`
              (`/Engine/EditorBlueprintResources/StandardMacros.IsValid` _returnvalue
                (:`Is Valid`
                  (message `/Game/Blueprints/Player/Bomberman_Interface.Planted Bomb Destroyed` _returnvalue))))
            (:`then_1`
              (`self.K2_DestroyActor`))))))))

(event `Draw Blast Particle`
  (params (`Hit Object Idx` :type Integer) (`Last Hit Actor Location` :type "Vector Structure") (`Trace Start Location` :type "Vector Structure") (`Trace End Location` :type "Vector Structure"))
  ;[1 1 1] Draw blast particle
  (bind _returnvalue (`GameplayStatics.SpawnEmitterAttached` "/Game/StarterContent/Particles/P_Explosion.P_Explosion" (`self.Bomb Mesh`) "None" (0.0 0.0 0.0) (struct) (1.0 1.0 1.0) "KeepRelativeOffset" false))
  (`ParticleSystemComponent.SetBeamSourcePoint` _returnvalue 0 `Trace Start Location` 0)
  (if (>= `Hit Object Idx` 0)
    (`ParticleSystemComponent.SetBeamTargetPoint` _returnvalue 0 `Last Hit Actor Location` 0)
    (else
      (`ParticleSystemComponent.SetBeamTargetPoint` _returnvalue 0 `Trace End Location` 0))))

(event `self.Bomb Mesh.OnComponentEndOverlap`
  (params (OverlappedComponent :type "PrimitiveComponent Object Reference") (OtherActor :type "Actor Object Reference") (OtherComp :type "PrimitiveComponent Object Reference") (OtherBodyIndex :type Integer))
  ;[1 1 1] Block Pawn when Owner moves away from the Bomb
  (bind _aspawn (cast `Pawn` OtherActor))
  (if (== _aspawn (`self.GetInstigator`))
    (`PrimitiveComponent.SetCollisionResponseToChannel` (`self.Bomb Mesh`) "ECC_Pawn" "ECR_Block")))

(fn `Blast In Direction`
  (params (Direction :type "Vector Structure"))
  (locals (`Is Destructible Wall` :type Boolean) (`Hit Object Idx` :type Integer :default -1) (`_Last Hit Actor Location` :type "Vector Structure"))
  (bind _returnvalue (`SceneComponent.K2_GetComponentLocation` (`self.Bomb Mesh`)))
  (bind _returnvalue_2 (+ _returnvalue (* Direction (`self.Blast Length`))))
  (bind _outhits (`KismetSystemLibrary.SphereTraceMultiForObjects` :`Start` _returnvalue :`End` _returnvalue_2 :`Radius` 10.0 :`ObjectTypes` (`|MakeArray` "ObjectTypeQuery6" "ObjectTypeQuery8" "ObjectTypeQuery7" "ObjectTypeQuery3" :!type "EObjectTypeQuery Enum") :`DrawDebugType` "Persistent" :`DrawTime` 1.0))
  (for (_array_element _array_index) _outhits
    (bind (_bblockinghit _binitialoverlap _time _distance _location _impactpoint _normal _impactnormal _physmat _hitactor) (`GameplayStatics.BreakHitResult` _array_element))
    (bind _output_get (set `local.Is Destructible Wall` (`.bSuccess` (cast `/Game/Blueprints/MapConstruction/DestructibleWall` _hitactor :!pure true)))) ; NOTE: Set it before interface call
    (if _output_get
      (set `local._Last Hit Actor Location` (+ _location (* Direction 50.0)))
      (else
        (set `local._Last Hit Actor Location` _location)))
    (bind _success (message `/Game/Blueprints/Weapon/WeaponInteract_Interface.Destroy` _hitactor))
    (if (or (not _success) (`local.Is Destructible Wall`))
      (set `local.Hit Object Idx` _array_index)
      (break)))
  ;[1 1 1] Draw blast particle
  (bind _returnvalue_3 (`GameplayStatics.SpawnEmitterAttached` "/Game/Effects/Particles/Beam/P_FireBlast.P_FireBlast" (`self.Bomb Mesh`) "None" (0.0 0.0 0.0) (struct) (1.0 1.0 1.0) "KeepRelativeOffset" false))
  (`ParticleSystemComponent.SetBeamSourcePoint` _returnvalue_3 0 _returnvalue 0)
  (if (>= (`local.Hit Object Idx`) 0)
    (`ParticleSystemComponent.SetBeamTargetPoint` _returnvalue_3 0 (`local._Last Hit Actor Location`) 0)
    (else
      (`ParticleSystemComponent.SetBeamTargetPoint` _returnvalue_3 0 _returnvalue_2 0))))

(fn `Destroy`
  (returns (Success :type Boolean))
  (`self.Explode`)
  (return true))

(fn `UserConstructionScript`)